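; Player Blueprint that extends an inherited forward trace with weapon effects and creates the player's UI widget on begin play.
; After the parent trace, a positive ChamberLine spawns a trail particle system from LineLocal to EndPoint.
; Otherwise it plays a no-ammo sound, with a Gate and one-second delay throttling repeats.
; SetCoolDown sets CoolDownOff to true after one second.
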(event `self.TraceForward`
  (`parent.TraceForward`)
  (if (> (`self.Chamber_Line`) 0)
    (bind _returnvalue (`NiagaraFunctionLibrary.SpawnSystemAtLocation` "/Game/Main/Assets/Particle/BulletTrail/PS_Trail_System.PS_Trail_System" (`SceneComponent.K2_GetComponentLocation` (`self.LineLocal`))))
    (`FXSystemComponent.SetVectorParameter` _returnvalue "End Point" (`self.EndPoint`))
    (else
      (`/Engine/EditorBlueprintResources/StandardMacros.Gate` false :!label _label
        (:`Exit`
          (`GameplayStatics.PlaySoundAtLocation` "/Game/Main/Assets/FirstPerson/Audio/153560__splicesound__winchester-rifle-cock-reload_No_Ammo_.153560__splicesound__winchester-rifle-cock-reload_No_Ammo_" (`self.K2_GetActorLocation`) (struct) 1.0 1.0 0.0 "/Game/Main/Assets/FirstPerson/Audio/FP_Sound_Auth.FP_Sound_Auth" null null)
          (`|ExecutionSequence`
            (:`then_0`
              (goto _label :!via `Close`))
            (:`then_1`
              (`KismetSystemLibrary.Delay` 1.0)
              (goto _label :!via `Open`))))))))

(event `self.ReceiveBeginPlay`
  (bind _returnvalue (`|CreateWidget` "/Game/Main/Blueprints/Player/BP_UI_Widget.BP_UI_Widget_C"))
  (bind _output_get (set `self.UI_Widget` _returnvalue))
  (`UserWidget.AddToViewport` _output_get 0))

(event `self.SetCoolDown`
  (`KismetSystemLibrary.Delay` 1.0)
  (set `self.CoolDownOff` true))

(fn `UserConstructionScript`)