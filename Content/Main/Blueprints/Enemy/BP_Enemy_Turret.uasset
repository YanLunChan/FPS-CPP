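; Enemy turret whose cylinder sweeps back and forth within a fixed yaw arc once the player overlaps its activation box.
; Every tick, even while inactive, it line-traces forward from an arrow and spawns a gunshot particle system ending at the hit location.
; A DoOnce destroys the first player character the trace hits.
; Any later box overlap by another actor switches rotation off, as activation is reassigned on each begin overlap.
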(event `self.ReceiveTick`
  (params (DeltaSeconds :type "Float (single-precision)"))
  (bind _cylinder (`self.Cylinder`))
  (bind _arrow (`self.Arrow`))
  (bind _returnvalue (`SceneComponent.K2_GetComponentLocation` _arrow))
  (bind _returnvalue_2 (* DeltaSeconds (`self.Rotation speed`)))
  (bind (_relativerotation_roll _relativerotation_pitch _relativerotation_yaw) (`KismetMathLibrary.BreakRotator` (`SceneComponent.RelativeRotation` (`self.Cylinder`))))
  (`|ExecutionSequence`
    (:`then_0`
      (if (`self.Activated`)
        (if (`self.Clockwise`)
          (`SceneComponent.K2_AddLocalRotation` _cylinder (`KismetMathLibrary.MakeRotator` 0.0 0.0 _returnvalue_2) false false)
          (else
            (`SceneComponent.K2_AddLocalRotation` _cylinder (`KismetMathLibrary.MakeRotator` 0.0 0.0 (* _returnvalue_2 -1.0)) false false)))))
    (:`then_1`
      (bind _outhit (`KismetSystemLibrary.LineTraceSingleForObjects` _returnvalue (+ _returnvalue (* (`SceneComponent.GetForwardVector` _arrow) (`self.distance`))) (`self.Object Types`)))
      (bind (_bblockinghit _binitialoverlap _time _distance _location _impactpoint _normal _impactnormal _physmat _hitactor _hitcomponent _hitbonename _hititem _elementindex _faceindex _tracestart) (`GameplayStatics.BreakHitResult` _outhit))
      (bind _returnvalue_3 (`NiagaraFunctionLibrary.SpawnSystemAtLocation` "/Game/Main/Assets/Particle/Mesh/LP_GunShot_System.LP_GunShot_System" _tracestart))
      (`FXSystemComponent.SetVectorParameter` _returnvalue_3 "End Point" _location)
      (bind _asplayer_character (cast `PlayerCharacter` _hitactor))
      (`/Engine/EditorBlueprintResources/StandardMacros.DoOnce` false
        (:`Completed`
          (`self.K2_DestroyActor` _asplayer_character))))
    (:`then_2`
      (if (not (and (>= _relativerotation_yaw -5.0) (<= _relativerotation_yaw 90.0)))
        (set `self.Clockwise` (not (`self.Clockwise`)))))))

(event `self.Activation box.OnComponentBeginOverlap`
  (params (OverlappedComponent :type "PrimitiveComponent Object Reference") (OtherActor :type "Actor Object Reference") (OtherComp :type "PrimitiveComponent Object Reference") (OtherBodyIndex :type Integer) (bFromSweep :type Boolean) (SweepResult :type "HitResult Structure (by ref)"))
  (set `self.Activated` (== OtherActor (`GameplayStatics.GetPlayerCharacter` 0))))

(fn `UserConstructionScript`)